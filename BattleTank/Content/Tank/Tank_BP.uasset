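; Tank pawn Blueprint that wires player input to the tank's aiming, movement and firing.
; On BeginPlay it initialises the TankAiming component with barrel and turret, and TankMovement with both tracks.
; Aim axes rotate an azimuth gimbal and spring arm, scaled by frame delta time.
; Tracks take direct per-track throttle or intent-based move and turn input through TankMovement, and the Fire action calls Fire.
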(event `self.ReceiveBeginPlay`
  (`KismetSystemLibrary.PrintString` "donkey: Tank BP BeginPlay")
  (`TankAimingComponent.Initialise` (`self.TankAiming`) (`self.Barrel`) (`self.Turret`))
  (`TankMovementComponent.Initialise` (`self.TankMovement`) (`self.LeftTrack`) (`self.RightTrack`)))

(event `InputAxis|AimAzimuth`
  (params (AxisValue :type "Float (single-precision)"))
  ;[1 1 1] Aim Bindings
  (`SceneComponent.K2_AddLocalRotation` (`self.Azimuth Gimball`) (`KismetMathLibrary.MakeRotator` 0.0 0.0 (* AxisValue (`GameplayStatics.GetWorldDeltaSeconds`) 100.0)) false false))

(event `InputAxis|Left Truck Throttle`
  (params (AxisValue :type "Float (single-precision)"))
  ;[1 1 1] Movement Input Binding
  (`TankTrack.SetTrackThrottle` (`self.LeftTrack`) AxisValue))

(event `InputAxis|Right Truck Throttle`
  (params (AxisValue :type "Float (single-precision)"))
  ;[1 1 1] Movement Input Binding
  (`TankTrack.SetTrackThrottle` (`self.RightTrack`) AxisValue))

(event `InputAxis|AimElevation`
  (params (AxisValue :type "Float (single-precision)"))
  ;[1 1 1] Aim Bindings
  (`SceneComponent.K2_AddLocalRotation` (`self.SpringArm`) (`KismetMathLibrary.MakeRotator` 0.0 (* AxisValue (`GameplayStatics.GetWorldDeltaSeconds`) 100.0)) false false))

(event `InputAxis|Move Forward`
  (params (AxisValue :type "Float (single-precision)"))
  ;[1 1 1] Movement Input Binding
  (`TankMovementComponent.IntentMoveForward` (`self.TankMovement`) AxisValue))

(event `InputAxis|Turn Right`
  (params (AxisValue :type "Float (single-precision)"))
  ;[1 1 1] Movement Input Binding
  (`TankMovementComponent.IntentTurnRight` (`self.TankMovement`) AxisValue))

(event `InputAction|Fire`
  (params (Key :type "Key Structure" :default "AnyKey"))
  ;[1 1 1] Aim Bindings
  (:`Pressed`
    (`self.Fire`)))

(event `InputAxis|Turn Left`
  (params (AxisValue :type "Float (single-precision)"))
  ;[1 1 1] Movement Input Binding
  (`TankMovementComponent.IntentTurnLeft` (`self.TankMovement`) AxisValue))

(event `InputAxis|Move Back`
  (params (AxisValue :type "Float (single-precision)"))
  ;[1 1 1] Movement Input Binding
  (`TankMovementComponent.IntentMoveBack` (`self.TankMovement`) AxisValue))

(fn `UserConstructionScript`
  (`KismetSystemLibrary.PrintString` "donkey: Tank_BP Construct"))